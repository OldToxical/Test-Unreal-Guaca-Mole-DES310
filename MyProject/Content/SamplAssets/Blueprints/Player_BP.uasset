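; Player character for a 2D side-scroller, built on a Paper2D flipbook sprite and character movement.
; Adds an Enhanced Input mapping context on BeginPlay for moving left, moving right and jumping.
; Movement runs along world X, and control rotation yaw flips to face the direction of travel.
; Each tick, the sprite's flipbook switches between jump, run and idle based on falling state and velocity.
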(event `self.ReceiveBeginPlay`
  (bind _asplayer_controller (cast `PlayerController` (`self.GetController`)))
  (bind _returnvalue (pcsubsystem `EnhancedInputLocalPlayerSubsystem` _asplayer_controller))
  (`/Engine/EditorBlueprintResources/StandardMacros.IsValid` _returnvalue
    (:`Is Valid`
      (`EnhancedInputSubsystemInterface.AddMappingContext` _returnvalue "/Game/SamplAssets/Input/NewInputMappingContext.NewInputMappingContext" 0 (struct)))))

(event `self.ReceiveTick`
  (params (DeltaSeconds :type "Float (single-precision)"))
  (`self.UpdateAnimation`))

(event `EnhancedInput|/Game/SamplAssets/Input/MoveLeft`
  (params (ActionValue :type Boolean) (ElapsedSeconds :type "Float (double-precision)") (TriggeredSeconds :type "Float (double-precision)") (InputAction :type "InputAction Object Reference" :default "/Game/SamplAssets/Input/MoveLeft.MoveLeft"))
  (:`Triggered`
    (`self.AddMovementInput` (-1.0 0.0 0.0))
    (`Controller.SetControlRotation` (`self.GetController`) (`KismetMathLibrary.MakeRotator` 0.0 0.0 180.0))))

(event `EnhancedInput|/Game/SamplAssets/Input/MoveRight`
  (params (ActionValue :type Boolean) (ElapsedSeconds :type "Float (double-precision)") (TriggeredSeconds :type "Float (double-precision)") (InputAction :type "InputAction Object Reference" :default "/Game/SamplAssets/Input/MoveRight.MoveRight"))
  (:`Triggered`
    (`self.AddMovementInput` (1.0 0.0 0.0))
    (`Controller.SetControlRotation` (`self.GetController`) (`KismetMathLibrary.MakeRotator` 0.0 0.0 0.0))))

(event `EnhancedInput|/Game/SamplAssets/Input/Jump`
  (params (ActionValue :type Boolean) (ElapsedSeconds :type "Float (double-precision)") (TriggeredSeconds :type "Float (double-precision)") (InputAction :type "InputAction Object Reference" :default "/Game/SamplAssets/Input/Jump.Jump"))
  (:`Triggered`
    (`self.Jump`)))

(event `UpdateAnimation`
  (`PaperFlipbookComponent.SetFlipbook` (`self.Sprite`) (select `bool` (`NavMovementComponent.IsFalling` (`self.CharacterMovement`)) :`false` (select `bool` (> (`KismetMathLibrary.VSize` (`MovementComponent.Velocity` (`self.CharacterMovement`))) 0.0) :`false` "/Game/SamplAssets/PNG/sprites/player/idle/player-idle.player-idle" :`true` "/Game/SamplAssets/PNG/sprites/player/run/player-run.player-run" :!type "PaperFlipbook Object Reference") :`true` "/Game/SamplAssets/PNG/sprites/player/jump/player-jump.player-jump")))

(fn `UserConstructionScript`)