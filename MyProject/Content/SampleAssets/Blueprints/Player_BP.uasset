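; Side-scrolling 2D player character with flipbook animation, horizontal movement and jumping.
; Left and right axis inputs add movement along world X and snap the controller yaw to face the sprite either way, while the Jump action triggers a jump.
; Every tick, UpdateAnimation picks the jump, run or idle flipbook from the movement component's falling state and velocity.
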(event `self.ReceiveTick`
  (params (DeltaSeconds :type "Float (single-precision)"))
  (`self.UpdateAnimation`))

(event `InputAxis|MoveLeft`
  (params (AxisValue :type "Float (single-precision)"))
  (`self.AddMovementInput` (-1.0 0.0 0.0) AxisValue)
  (`Controller.SetControlRotation` (`self.GetController`) (`KismetMathLibrary.MakeRotator` 0.0 0.0 0.0)))

(event `InputAxis|MoveRight`
  (params (AxisValue :type "Float (single-precision)"))
  (`self.AddMovementInput` (1.0 0.0 0.0) AxisValue)
  (`Controller.SetControlRotation` (`self.GetController`) (`KismetMathLibrary.MakeRotator` 0.0 0.0 180.0)))

(event `InputAction|Jump`
  (params (Key :type "Key Structure"))
  (:`Pressed`
    (`self.Jump`)))

(event `UpdateAnimation`
  (`PaperFlipbookComponent.SetFlipbook` (`self.Sprite`) (select `bool` (`NavMovementComponent.IsFalling` (`self.CharacterMovement`)) :`false` (select `bool` (> (`KismetMathLibrary.VSize` (`MovementComponent.Velocity` (`self.CharacterMovement`))) 0.0) :`false` "/Game/SampleAssets/PNG/sprites/player/idle/player-idle.player-idle" :`true` "/Game/SampleAssets/PNG/sprites/player/run/player-run.player-run" :!type "PaperFlipbook Object Reference") :`true` "/Game/SampleAssets/PNG/sprites/player/jump/player-jump.player-jump")))

(fn `UserConstructionScript`)